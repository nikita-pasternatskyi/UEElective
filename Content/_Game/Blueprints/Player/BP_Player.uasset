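; BP_Player is the player character Blueprint, holding an unfinished ledge-detection check that no event triggers.
; While in the air, it line-traces forward from the capsule's top front edge to find a wall.
; A capsule-sized trace above the probe end then tests for standing room.
; If that space is clear, movement stops and switches to Flying; no climb motion follows.
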(fn `UserConstructionScript`)