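; Player state for walking, one state in the character's state machine, which caps the movement component's max walk speed on entry.
; Each tick it feeds move input to the owning character's Move function.
; It then switches to Idle when input is near zero, or to Jump, Slide or Jog when the jump, slide or sprint input is just pressed.
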(event `self.TickState`
  (params (deltaTime :type "Float (single-precision)"))
  (`|ExecutionSequence`
    (:`then_0`
      ;[1 1 1] Move
      (`UEElectiveCharacter.Move` (`self.m_OwningCharacter`) (`self.GetMoveInput`)))
    (:`then_1`
      ;[1 1 1] SwitchToIdle
      (if (== (`self.GetMoveInput`) (0.0 0.0) :`ErrorTolerance` 0.1)
        (`StateMachineComponent.ChangeState` (`self.m_StateMachine`) "/Game/_Game/Blueprints/Player/States/BP_PlayerState_Idle.BP_PlayerState_Idle_C")))
    (:`then_2`
      ;[1 1 1] Change to Jump State
      (if (`.JustPressed` (break `PlayerInputActionState` (`PlayerInputStamp.JumpValue` (`self.m_PlayerInput`))))
        (`StateMachineComponent.ChangeState` (`self.m_StateMachine`) "/Game/_Game/Blueprints/Player/States/BP_PlayerState_Jump.BP_PlayerState_Jump_C")))
    (:`then_3`
      ;[1 1 1] Change to Slide State
      (if (`.JustPressed` (break `PlayerInputActionState` (`PlayerInputStamp.SlideValue` (`self.m_PlayerInput`))))
        (`StateMachineComponent.ChangeState` (`self.m_StateMachine`) "/Game/_Game/Blueprints/Player/States/BP_PlayerState_Slide.BP_PlayerState_Slide_C")))
    (:`then_4`
      ;[1 1 1] Change to Slide State
      (if (`.JustPressed` (break `PlayerInputActionState` (`PlayerInputStamp.SprintValue` (`self.m_PlayerInput`))))
        (`StateMachineComponent.ChangeState` (`self.m_StateMachine`) "/Game/_Game/Blueprints/Player/States/BP_PlayerState_Jog.BP_PlayerState_Jog_C")))))

(fn `StateEntered`
  (set `CharacterMovementComponent.MaxWalkSpeed` 200.0 (`Character.CharacterMovement` (`self.m_OwningCharacter`))))