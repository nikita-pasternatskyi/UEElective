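; Base class for player states, providing shared camera setup and movement input helpers.
; On entering, it applies its CameraSettings through the owning character's CameraTransitioner, then calls StateEntered, an empty hook.
; Helper functions return normalized 2D move input and a world-space direction built from the controller's full control rotation, so pitch is not flattened out.
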(event `self.EnterState`
  (`CameraTransitionerComponent.ChangeCameraSettingsState` (`UEElectiveCharacter.CameraTransitioner` (`self.m_OwningCharacter`)) (`self.CameraSettings`))
  (`self.StateEntered`))

(fn `GetMoveInput`
  (returns (Input :type "Vector2D Structure"))
  (bind (_x _y) (`EnhancedInputLibrary.BreakInputActionValue` (`.InputValue` (break `PlayerInputActionState` (`PlayerInputStamp.MoveValue` (`self.m_PlayerInput`))))))
  (return (`KismetMathLibrary.Normal2D` (`KismetMathLibrary.MakeVector2D` _x _y))))

(fn `GetVector3RelativeMoveInput`
  (returns (MoveInput :type "Vector Structure"))
  (bind (_x _y) (`KismetMathLibrary.BreakVector2D` (`self.GetMoveInput`)))
  (bind _returnvalue (`Controller.GetControlRotation` (`Pawn.GetController` (`self.m_OwningCharacter`))))
  (return (`KismetMathLibrary.Normal` (+ (* (`KismetMathLibrary.GetRightVector` _returnvalue) _x) (* (`KismetMathLibrary.GetForwardVector` _returnvalue) _y)))))

(fn `StateEntered`)