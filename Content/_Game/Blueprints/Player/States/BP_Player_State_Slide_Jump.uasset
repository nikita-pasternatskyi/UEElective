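; Player state for a slide jump that orients the character's mesh along its flight path.
; Each tick it builds a world rotation from the velocity direction, with a -90 yaw offset and swapped pitch and roll, then switches to Idle on landing.
; Exiting restores the mesh's default relative rotation.
; Jump release and air movement logic is present but unconnected, so this graph applies neither.
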(event `self.TickState`
  (params (deltaTime :type "Float (single-precision)"))
  (`|ExecutionSequence`
    (:`then_0`
      (`SceneComponent.K2_SetWorldRotation` (`Character.Mesh` (`self.m_OwningCharacter`)) (`KismetMathLibrary.MakeRotator` (* (.pitch (`KismetMathLibrary.ComposeRotators` (`KismetMathLibrary.MakeRotFromX` (`KismetMathLibrary.Normal` (`Actor.GetVelocity` (`self.m_OwningCharacter`)))) (`KismetMathLibrary.MakeRotator` 0.0 0.0 -90.0))) -1.0) (.roll (`KismetMathLibrary.ComposeRotators` (`KismetMathLibrary.MakeRotFromX` (`KismetMathLibrary.Normal` (`Actor.GetVelocity` (`self.m_OwningCharacter`)))) (`KismetMathLibrary.MakeRotator` 0.0 0.0 -90.0))) (.yaw (`KismetMathLibrary.ComposeRotators` (`KismetMathLibrary.MakeRotFromX` (`KismetMathLibrary.Normal` (`Actor.GetVelocity` (`self.m_OwningCharacter`)))) (`KismetMathLibrary.MakeRotator` 0.0 0.0 -90.0)))) false false))
    (:`then_1`
      (if (`NavMovementComponent.IsMovingOnGround` (`Character.CharacterMovement` (`self.m_OwningCharacter`)))
        (`StateMachineComponent.ChangeState` (`self.m_StateMachine`) "/Game/_Game/Blueprints/Player/States/BP_PlayerState_Idle.BP_PlayerState_Idle_C")))))

(event `self.ExitState`
  (`SceneComponent.K2_SetRelativeRotation` (`Character.Mesh` (`self.m_OwningCharacter`)) (struct :`Yaw` -90.0) false false))