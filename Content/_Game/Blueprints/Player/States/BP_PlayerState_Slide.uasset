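; Player state for sliding, run by the player state machine.
; On entry it picks a direction from move input, or actor forward without input, and sets velocity to slide force plus current horizontal speed.
; Each tick, a jump press launches the character along move input with added upward velocity and switches to Slide Jump.
; It switches to Idle when input is near zero and the character is grounded with no horizontal velocity.
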(event `self.TickState`
  (params (deltaTime :type "Float (single-precision)"))
  (`|ExecutionSequence`
    (:`then_0`
      ;[1 1 1] Slide Jump
      (if (`.JustPressed` (break `PlayerInputActionState` (`PlayerInputStamp.JumpValue` (`self.m_PlayerInput`))))
        (bind _moveinput (`self.GetVector3RelativeMoveInput`))
        (`Character.LaunchCharacter` (`self.m_OwningCharacter`) (+ (* _moveinput (`self.SlideForce`)) (`KismetMathLibrary.MakeVector` 0.0 0.0 (`self.SlideForceJumpMultiplier`))) true true) ; To-Do: Enable onland switch to idle/whatever
        (`StateMachineComponent.ChangeState` (`self.m_StateMachine`) "/Game/_Game/Blueprints/Player/States/BP_PlayerState_Slide_Jump.BP_PlayerState_Slide_Jump_C")))
    (:`then_1`
      ;[1 1 1] SwitchToIdle
      (if (== (`self.GetMoveInput`) (0.0 0.0) :`ErrorTolerance` 0.1)
        (if (== (`KismetMathLibrary.VSizeXY` (`Actor.GetVelocity` (`self.m_OwningCharacter`))) 0.0)
          (if (`NavMovementComponent.IsMovingOnGround` (`Character.CharacterMovement` (`self.m_OwningCharacter`)))
            (`StateMachineComponent.ChangeState` (`self.m_StateMachine`) "/Game/_Game/Blueprints/Player/States/BP_PlayerState_Idle.BP_PlayerState_Idle_C")))))))

(fn `StateEntered`
  (`|ExecutionSequence`
    (:`then_0`
      ;[1 1 1] Calculate Slide Direction
      (if (== (`self.GetMoveInput`) (0.0 0.0))
        (set `self.SlideDirection` (`Actor.GetActorForwardVector` (`self.m_OwningCharacter`)))
        (else
          (bind _moveinput (`self.GetVector3RelativeMoveInput`))
          (set `self.SlideDirection` _moveinput))))
    (:`then_1`
      ;[1 1 1] Slide Push
      (set `MovementComponent.Velocity` (* (`self.SlideDirection`) (+ (`self.SlideForce`) (`KismetMathLibrary.VSizeXY` (`CharacterMovementComponent.GetLastUpdateVelocity` (`Character.CharacterMovement` (`self.m_OwningCharacter`)))))) (`Character.CharacterMovement` (`self.m_OwningCharacter`))))))