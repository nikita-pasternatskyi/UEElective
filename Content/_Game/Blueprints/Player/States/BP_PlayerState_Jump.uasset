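; Player state in a state machine that handles the character's jump and time in the air.
; On enter it starts the jump on the owning character.
; Each tick it stops jumping when the jump input is released, switches to the Idle state once the movement component is on the ground, and applies move input for air control.
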(event `self.EnterState`
  (`Character.Jump` (`self.m_OwningCharacter`)))

(event `self.TickState`
  (params (deltaTime :type "Float (single-precision)"))
  (`|ExecutionSequence`
    (:`then_0`
      ;[1 1 1] Stop Jump
      (if (`.JustReleased` (break `PlayerInputActionState` (`PlayerInputStamp.JumpValue` (`self.m_PlayerInput`))))
        (`Character.StopJumping` (`self.m_OwningCharacter`))))
    (:`then_1`
      ;[1 1 1] SwitchToGround
      (if (`NavMovementComponent.IsMovingOnGround` (`Character.CharacterMovement` (`self.m_OwningCharacter`)))
        (`StateMachineComponent.ChangeState` (`self.m_StateMachine`) "/Game/_Game/Blueprints/Player/States/BP_PlayerState_Idle.BP_PlayerState_Idle_C")))
    (:`then_2`
      ;[1 1 1] InAir Movement
      (`UEElectiveCharacter.Move` (`self.m_OwningCharacter`) (`self.GetMoveInput`)))))